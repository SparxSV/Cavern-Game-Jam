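; BP_WideGolem is an AI golem pawn that wanders until it spots the player, then chases and attacks.
; While it has not seen the player, Tick issues moves to random reachable points around it.
; PawnSensing sets a seen flag and starts a chase, playing the wide attack montage on arrival behind a brief CanAttack delay.
; Once set, the seen flag never effectively clears, so wandering does not resume.
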(event OnSeePawn(PawnSensing)
  (params (Pawn :type Pawn%20Object%20Reference))
  (Variables|Default|SetIsSeeingPlayer true)
  (CallFunction|FollowPlayer))

(event Custom|FollowPlayer
  (Variables|Default|SetCanAttack true)
  (if (Variables|Default|GetIsSeeingPlayer)
    (AI|AIMoveTo self "0, 0, 0" (Game|GetPlayerCharacter 0) 7e+01 false
      (:OnSuccess
        (if (Variables|Default|GetCanAttack)
          (Variables|Default|SetCanAttack false)
          (Animation|PlayAnimMontage "/Game/AI/Animations/AM_WideAttack.AM_WideAttack" 1.0 "None")
          (Utilities|FlowControl|Delay 0.2)
          (Variables|Default|SetCanAttack true))))
    (else
      (Variables|Default|SetIsSeeingPlayer false))))

(event EventBeginPlay)

(event EventTick
  (params (DeltaSeconds :type Float%20%28single-precision%29))
  (bind _self self)
  (if (not (Variables|Default|GetIsSeeingPlayer))
    (AI|AIMoveTo _self (.RandomLocation (AI|Navigation|GetRandomReachablePointinRadius (Transformation|GetActorLocation _self) 1e+03 0 0)) 0 1.2e+02 false)))

(fn ConstructionScript)